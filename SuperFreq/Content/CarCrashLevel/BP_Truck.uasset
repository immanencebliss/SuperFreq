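; BP_Truck is a truck actor in the car crash level that drives itself along a road spline.
; On BeginPlay, if ActiveCar is set, a timeline starts from a configurable start offset with its play rate scaled by Duration.
; Each update maps the timeline alpha to a distance along the RoadTrack spline and applies that world location and rotation, with fixed world-Y and yaw offsets.
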(event `self.ReceiveBeginPlay`
  (if (`self.ActiveCar`)
    (`self.MoveCar`)))

(event `MoveCar`
  (bind _returnvalue (`KismetMathLibrary.Lerp` 0.0 (`SplineComponent.GetSplineLength` (`/Game/CarCrashLevel/RoadSpline.Spline` (`self.RoadTrack`))) (`self.Alpha`)))
  (bind (_returnvalue_x _returnvalue_y _returnvalue_z) (`KismetMathLibrary.BreakVector` (`SplineComponent.GetLocationAtDistanceAlongSpline` (`/Game/CarCrashLevel/RoadSpline.Spline` (`self.RoadTrack`)) _returnvalue "World")))
  (bind (_returnvalue_roll _returnvalue_pitch _returnvalue_yaw) (`KismetMathLibrary.BreakRotator` (`SplineComponent.GetRotationAtDistanceAlongSpline` (`/Game/CarCrashLevel/RoadSpline.Spline` (`self.RoadTrack`)) _returnvalue "World")))
  (`TimelineComponent.SetPlayRate` (`self.CarMover`) (/ 1.0 (`self.Duration`)))
  (`TimelineComponent.SetNewTime` (`self.CarMover`) (`self.CarStartOffset`))
  (bind (_direction _alpha) (`Timeline|CarMover`)
    (:`Update`
      (set `self.Alpha` _alpha)
      (`self.K2_SetActorLocationAndRotation` (`KismetMathLibrary.MakeVector` _returnvalue_x (+ _returnvalue_y 300.0) _returnvalue_z) (`KismetMathLibrary.MakeRotator` _returnvalue_roll _returnvalue_pitch (+ _returnvalue_yaw -90.0))))))

(fn `UserConstructionScript`)