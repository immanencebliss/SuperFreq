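; Mystery machine prop with a glitching screen, flickering lights and two constantly rotating scene components.
; If ShouldFlicker is set, BeginPlay creates dynamic materials for screen and lights, then starts two randomly timed, self-restarting loops.
; Flicker drives light brightness through one of three random timelines, while ScreenError swaps random error or horror flipbook textures with matching grid and speed parameters.
; Tick rotates the scene components by a fixed per-frame step, independent of delta time.
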(event `Flicker`
  (`KismetSystemLibrary.Delay` (`KismetMathLibrary.RandomFloatInRange` 0.5 2.8))
  (switch `int` (`KismetMathLibrary.RandomIntegerInRange` 0 2)
    (:`0`
      (bind (_direction _alpha) (`Timeline|Timeline_0` :!via `PlayFromStart`)
        (:`Update`
          (`MaterialInstanceDynamic.SetScalarParameterValue` (`self.Lights`) "Brightness" (`KismetMathLibrary.Lerp` 3.0 0.0 _alpha)))
        (:`Finished`
          (`self.Flicker`))))
    (:`1`
      (bind (_direction_2 _alpha_2) (`Timeline|Timeline_1` :!via `PlayFromStart`)
        (:`Update`
          (`MaterialInstanceDynamic.SetScalarParameterValue` (`self.Lights`) "Brightness" (`KismetMathLibrary.Lerp` 3.0 0.0 _alpha_2)))
        (:`Finished`
          (`self.Flicker`))))
    (:`2`
      (bind (_direction_3 _alpha_3) (`Timeline|Timeline_2` :!via `PlayFromStart`)
        (:`Update`
          (`MaterialInstanceDynamic.SetScalarParameterValue` (`self.Lights`) "Brightness" (`KismetMathLibrary.Lerp` 3.0 0.0 _alpha_3)))
        (:`Finished`
          (`self.Flicker`))))))

(event `ScreenError`
  (`KismetSystemLibrary.Delay` (`KismetMathLibrary.RandomFloatInRange` 0.5 3.0))
  (switch `int` (`KismetMathLibrary.RandomIntegerInRange` 0 10)
    (:`Default`
      (set `self.Texture` "/Game/IanTextures/fatalerror.fatalerror")
      (set `self.Rows` 2.0)
      (set `self.Columns` 19.0)
      (set `self.Speed` 1.0))
    (:`0`
      (set `self.Texture` "/Game/IanTextures/Failure.Failure")
      (set `self.Rows` 3.0)
      (set `self.Columns` 5.0)
      (set `self.Speed` 1.0))
    (:`1`
      (set `self.Texture` "/Game/IanTextures/icant.icant")
      (set `self.Rows` 2.0)
      (set `self.Columns` 7.0)
      (set `self.Speed` 1.0))
    (:`2`
      (set `self.Texture` "/Game/IanTextures/mouthblood.mouthblood")
      (set `self.Rows` 3.0)
      (set `self.Columns` 5.0)
      (set `self.Speed` 1.0))
    (:`3`
      (set `self.Texture` "/Game/IanTextures/MouthClamp.MouthClamp")
      (set `self.Rows` 3.0)
      (set `self.Columns` 3.0)
      (set `self.Speed` 1.0))
    (:`4`
      (set `self.Texture` "/Game/IanTextures/noise.noise")
      (set `self.Rows` 3.0)
      (set `self.Columns` 3.0)
      (set `self.Speed` 1.0))
    (:`5`
      (set `self.Texture` "/Game/IanTextures/eyeball.eyeball")
      (set `self.Rows` 3.0)
      (set `self.Columns` 31.0)
      (set `self.Speed` 0.25))
    (:`6`
      (set `self.Texture` "/Game/IanTextures/rage.rage")
      (set `self.Rows` 4.0)
      (set `self.Columns` 5.0)
      (set `self.Speed` 1.0))
    (:`7`
      (set `self.Texture` "/Game/IanTextures/donttouch.donttouch")
      (set `self.Rows` 6.0)
      (set `self.Columns` 12.0)
      (set `self.Speed` 1.0))
    (:`8`
      (set `self.Texture` "/Game/IanTextures/die.die")
      (set `self.Rows` 2.0)
      (set `self.Columns` 2.0)
      (set `self.Speed` 3.0)))
  (`MaterialInstanceDynamic.SetTextureParameterValue` (`self.Screen`) "Texture" (`self.Texture`))
  (`MaterialInstanceDynamic.SetScalarParameterValue` (`self.Screen`) "Rows" (`self.Rows`))
  (`MaterialInstanceDynamic.SetScalarParameterValue` (`self.Screen`) "Columns" (`self.Columns`))
  (`MaterialInstanceDynamic.SetScalarParameterValue` (`self.Screen`) "Speed" (`self.Speed`))
  (`self.ScreenError`))

(event `self.ReceiveBeginPlay`
  (if (`self.ShouldFlicker`)
    (bind _returnvalue (`PrimitiveComponent.CreateDynamicMaterialInstance` (`self.mystery_machine_for_blueprints`) 3 "/Game/IanTextures/Mat_Haxor.Mat_Haxor" "None"))
    (set `self.Screen` _returnvalue)
    (bind _returnvalue_2 (`PrimitiveComponent.CreateDynamicMaterialInstance` (`self.mystery_machine_for_blueprints`) 2 "/Game/Models/Kristian/Mystery_Machine/Texture_MOD_A_MYSTERY_MACHINE_AND_HOOD/BMM_Computer01_Buttons_Dials_BaseColor_Mat.BMM_Computer01_Buttons_Dials_BaseColor_Mat" "None"))
    (set `self.Lights` _returnvalue_2)
    (`self.Flicker`)
    (`self.ScreenError`)))

(event `self.ReceiveTick`
  (params (DeltaSeconds :type "Float (single-precision)"))
  (`|ExecutionSequence`
    (:`then_0`
      (`SceneComponent.K2_AddLocalRotation` (`self.Scene`) (struct :`Roll` 0.5) false false))
    (:`then_1`
      (`SceneComponent.K2_AddLocalRotation` (`self.Scene1`) (struct :`Roll` 0.5) false false))))

(fn `UserConstructionScript`)