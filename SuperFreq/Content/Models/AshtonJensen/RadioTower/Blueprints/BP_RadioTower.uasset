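; BP_RadioTower is a radio tower prop with a blinking light on its Sphere component.
; On BeginPlay it creates a dynamic Blink material instance and starts a timer with a random initial delay.
; Each blink plays a timeline that drives the Brightness parameter up to MaxBrightness via a lerp, then schedules the next blink after another random delay, forming an endless irregular cycle.
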(event `self.ReceiveBeginPlay`
  (bind _returnvalue (`PrimitiveComponent.CreateDynamicMaterialInstance` (`self.Sphere`) 0 "/Game/SpringLandscape/Blink.Blink" "None"))
  (set `self.MatInst` _returnvalue)
  (`KismetSystemLibrary.K2_SetTimerDelegate` (delegate `Blink`) (`KismetMathLibrary.RandomFloatInRange` 0.0 5.0)))

(event `Blink`
  (bind (_direction _alpha) (`Timeline|BlinkTL` :!via `PlayFromStart`)
    (:`Update`
      (`MaterialInstanceDynamic.SetScalarParameterValue` (`self.MatInst`) "Brightness" (`KismetMathLibrary.Lerp` 0.0 (`self.MaxBrightness`) _alpha)))
    (:`Finished`
      (`KismetSystemLibrary.K2_SetTimerDelegate` (delegate `Blink`) (`KismetMathLibrary.RandomFloatInRange` 3.0 5.0)))))

(fn `UserConstructionScript`)