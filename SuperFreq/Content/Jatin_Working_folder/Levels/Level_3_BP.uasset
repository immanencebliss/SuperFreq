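; Level 3 wire-routing puzzle: the player steers three cable chains through waypoints and connectors to their end points, then the next level opens.
; On Tick, a pair of HUD widget sliders per wire moves the active cable segment's end in X and Z.
; Reaching each target within tolerance latches a flag and reveals the next segment; the last activates end effects.
; BeginPlay hides later segments and effects, assigns materials and caches the HUD.
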(event `self.ReceiveTick`
  (params (DeltaSeconds :type "Float (single-precision)"))
  (bind _cable_1_2 (`self.Cable_1_2`))
  (bind _cable_6 (`self.Cable_6`))
  (bind _cable_1 (`self.Cable_1`))
  (bind _cable_2_2 (`self.Cable_2_2`))
  (bind _cable_4 (`self.Cable_4`))
  (bind _cable_6_2 (`self.Cable_6_2`))
  (bind _cable_2 (`self.Cable_2`))
  (bind _cable_3_2 (`self.Cable_3_2`))
  (bind _cable_5 (`self.Cable_5`))
  (bind _cable_4_2 (`self.Cable_4_2`))
  (bind _cable_5_2 (`self.Cable_5_2`))
  (bind _cable_3 (`self.Cable_3`))
  (bind (_endlocation_x _endlocation_y) (`KismetMathLibrary.BreakVector` (`CableComponent.EndLocation` _cable_1_2)))
  (bind (_endlocation_x_2 _endlocation_y_2) (`KismetMathLibrary.BreakVector` (`CableComponent.EndLocation` _cable_6)))
  (bind (_endlocation_x_3 _endlocation_y_3) (`KismetMathLibrary.BreakVector` (`CableComponent.EndLocation` _cable_1)))
  (bind (_endlocation_x_4 _endlocation_y_4) (`KismetMathLibrary.BreakVector` (`CableComponent.EndLocation` _cable_2_2)))
  (bind (_endlocation_x_5 _endlocation_y_5) (`KismetMathLibrary.BreakVector` (`CableComponent.EndLocation` _cable_4)))
  (bind (_endlocation_x_6 _endlocation_y_6) (`KismetMathLibrary.BreakVector` (`CableComponent.EndLocation` _cable_6_2)))
  (bind (_endlocation_x_7 _endlocation_y_7) (`KismetMathLibrary.BreakVector` (`CableComponent.EndLocation` _cable_2)))
  (bind (_endlocation_x_8 _endlocation_y_8) (`KismetMathLibrary.BreakVector` (`CableComponent.EndLocation` _cable_3_2)))
  (bind (_endlocation_x_9 _endlocation_y_9) (`KismetMathLibrary.BreakVector` (`CableComponent.EndLocation` _cable_5)))
  (bind (_endlocation_x_10 _endlocation_y_10) (`KismetMathLibrary.BreakVector` (`CableComponent.EndLocation` _cable_4_2)))
  (bind (_endlocation_x_11 _endlocation_y_11) (`KismetMathLibrary.BreakVector` (`CableComponent.EndLocation` _cable_5_2)))
  (bind (_endlocation_x_12 _endlocation_y_12) (`KismetMathLibrary.BreakVector` (`CableComponent.EndLocation` _cable_3)))
  (`|ExecutionSequence`
    (:`then_0`
      ;[1 1 1] Wire 1 Start To End 1->1
      (if (`self.Key_1_1`)
        (if (`self.Connector_1_CC`)
          (if (`self.Key_1_2`)
            (if (not (`self.End_1_CC`))
              (bind _next_level_wd (`/Game/Jatin_Working_folder/HUD/Next_Level_HUD.Next_Level_WD` (stale `self.ReceiveBeginPlay` _asnext_level_hud)))
              (bind _slider_2_value (`/Game/Jatin_Working_folder/Widgets/Player_UI.Slider_2_Value` _next_level_wd))
              (bind _slider_1_value (`/Game/Jatin_Working_folder/Widgets/Player_UI.Slider_1_Value` _next_level_wd))
              (bind _output_get (set `CableComponent.EndLocation` (`KismetMathLibrary.MakeVector` (- (* _slider_2_value 200.0) 425.0) _endlocation_y_6 (* _slider_1_value 200.0)) _cable_6_2))
              (if (== _output_get (`SceneComponent.RelativeLocation` (`self.End_2`)) :`ErrorTolerance` 30.0)
                (set `self.End_1_CC` true)
                (`ActorComponent.SetActive` (`self.End_PS_2`) true false)
                (`ActorComponent.SetActive` (`self.End_PT_2`) true false)))
            (else
              (bind _output_get_2 (set `CableComponent.EndLocation` (`KismetMathLibrary.MakeVector` (- (* _slider_2_value 200.0) 425.0) _endlocation_y_5 (* _slider_1_value 200.0)) _cable_4))
              (if (== _output_get_2 (`SceneComponent.RelativeLocation` (`self.6`)) :`ErrorTolerance` 30.0)
                (set `self.Key_1_2` true)
                (`SceneComponent.SetVisibility` (`self.Cable_6_2`) true false))))
          (else
            (bind _output_get_3 (set `CableComponent.EndLocation` (`KismetMathLibrary.MakeVector` (- (* _slider_2_value 200.0) 425.0) _endlocation_y_4 (* _slider_1_value 200.0)) _cable_2_2))
            (if (== _output_get_3 (`SceneComponent.RelativeLocation` (`self.Connector_1`)) :`ErrorTolerance` 20.0)
              (set `self.Connector_1_CC` true)
              (`SceneComponent.SetVisibility` (`self.Cable_4`) true false))))
        (else
          (bind _output_get_4 (set `CableComponent.EndLocation` (`KismetMathLibrary.MakeVector` (- (* _slider_2_value 200.0) 425.0) _endlocation_y_3 (* _slider_1_value 200.0)) _cable_1))
          (if (== _output_get_4 (`SceneComponent.RelativeLocation` (`self.2`)) :`ErrorTolerance` 20.0)
            (set `self.Key_1_1` true)
            (`SceneComponent.SetVisibility` (`self.Cable_2_2`) true false)))))
    (:`then_1`
      ;[1 1 1] Wire 2 Start To End 1->1
      (if (`self.Key_2_1`)
        (if (`self.Connector_2_cc`)
          (if (`self.Key_2_2`)
            (if (not (`self.End_2_cc`))
              (bind _slider_4_value (`/Game/Jatin_Working_folder/Widgets/Player_UI.Slider_4_Value` _next_level_wd))
              (bind _slider_3_value (`/Game/Jatin_Working_folder/Widgets/Player_UI.Slider_3_Value` _next_level_wd))
              (bind _output_get_5 (set `CableComponent.EndLocation` (`KismetMathLibrary.MakeVector` (- (* _slider_4_value 200.0) 425.0) _endlocation_y_10 (* _slider_3_value 200.0)) _cable_4_2))
              (if (== _output_get_5 (`SceneComponent.RelativeLocation` (`self.End_1`)) :`ErrorTolerance` 30.0)
                (set `self.End_2_cc` true)
                (`ActorComponent.SetActive` (`self.End_PS_1`) true false)
                (`ActorComponent.SetActive` (`self.End_PT_1`) true false)))
            (else
              (bind _output_get_6 (set `CableComponent.EndLocation` (`KismetMathLibrary.MakeVector` (- (* _slider_4_value 200.0) 425.0) _endlocation_y_9 (* _slider_3_value 200.0)) _cable_5))
              (if (== _output_get_6 (`SceneComponent.RelativeLocation` (`self.4`)) :`ErrorTolerance` 30.0)
                (set `self.Key_2_2` true)
                (`SceneComponent.SetVisibility` (`self.Cable_4_2`) true false))))
          (else
            (bind _output_get_7 (set `CableComponent.EndLocation` (`KismetMathLibrary.MakeVector` (- (* _slider_4_value 200.0) 425.0) _endlocation_y_8 (* _slider_3_value 200.0)) _cable_3_2))
            (if (== _output_get_7 (`SceneComponent.RelativeLocation` (`self.Connector_2`)) :`ErrorTolerance` 20.0)
              (set `self.Connector_2_cc` true)
              (`SceneComponent.SetVisibility` (`self.Cable_5`) true false))))
        (else
          (bind _output_get_8 (set `CableComponent.EndLocation` (`KismetMathLibrary.MakeVector` (- (* _slider_4_value 200.0) 425.0) _endlocation_y_7 (* _slider_3_value 200.0)) _cable_2))
          (if (== _output_get_8 (`SceneComponent.RelativeLocation` (`self.3`)) :`ErrorTolerance` 20.0)
            (set `self.Key_2_1` true)
            (`SceneComponent.SetVisibility` (`self.Cable_3_2`) true false)))))
    (:`then_2`
      ;[1 1 1] Wire 3 Start To End 1->1
      (if (`self.Key_3_1`)
        (if (`self.Connector_3_cc`)
          (if (`self.Key_3_2`)
            (if (not (`self.End_3_cc`))
              (bind _slider_5_value (`/Game/Jatin_Working_folder/Widgets/Player_UI.Slider_5_Value` _next_level_wd))
              (bind _slider_6_value (`/Game/Jatin_Working_folder/Widgets/Player_UI.Slider_6_Value` _next_level_wd))
              (bind _output_get_9 (set `CableComponent.EndLocation` (`KismetMathLibrary.MakeVector` (- (* _slider_5_value 200.0) 425.0) _endlocation_y_11 (* _slider_6_value 200.0)) _cable_5_2))
              (if (== _output_get_9 (`SceneComponent.RelativeLocation` (`self.End_3`)) :`ErrorTolerance` 30.0)
                (set `self.End_3_cc` true)
                (`ActorComponent.SetActive` (`self.End_PS_3`) true false)
                (`ActorComponent.SetActive` (`self.End_PT_3`) true false)))
            (else
              (bind _output_get_10 (set `CableComponent.EndLocation` (`KismetMathLibrary.MakeVector` (- (* _slider_5_value 200.0) 425.0) _endlocation_y_2 (* _slider_6_value 200.0)) _cable_6))
              (if (== _output_get_10 (`SceneComponent.RelativeLocation` (`self.5`)) :`ErrorTolerance` 30.0)
                (set `self.Key_3_2` true)
                (`SceneComponent.SetVisibility` (`self.Cable_5_2`) true false))))
          (else
            (bind _output_get_11 (set `CableComponent.EndLocation` (`KismetMathLibrary.MakeVector` (- (* _slider_5_value 200.0) 425.0) _endlocation_y (* _slider_6_value 200.0)) _cable_1_2))
            (if (== _output_get_11 (`SceneComponent.RelativeLocation` (`self.Connector_3`)) :`ErrorTolerance` 20.0)
              (set `self.Connector_3_cc` true)
              (`SceneComponent.SetVisibility` (`self.Cable_6`) true false))))
        (else
          (bind _output_get_12 (set `CableComponent.EndLocation` (`KismetMathLibrary.MakeVector` (- (* _slider_5_value 200.0) 425.0) _endlocation_y_12 (* _slider_6_value 200.0)) _cable_3))
          (if (== _output_get_12 (`SceneComponent.RelativeLocation` (`self.1`)) :`ErrorTolerance` 20.0)
            (set `self.Key_3_1` true)
            (`SceneComponent.SetVisibility` (`self.Cable_1_2`) true false)))))
    (:`then_3`
      (if (and (`self.End_1_CC`) (`self.End_2_cc`) (`self.End_3_cc`))
        (`GameplayStatics.OpenLevel` (`self.LevelToLoad`))))))

(event `self.ReceiveBeginPlay`
  (bind _mat_for_start_1 (`self.Mat for Start 1`))
  (bind _mat_for_start_2 (`self.Mat for Start 2`))
  (bind _mat_for_start_3 (`self.Mat for Start 3`))
  (bind _mat_for_obt_2 (`self.Mat for Obt_2`))
  (bind _mat_for_obt_3 (`self.Mat for Obt_3`))
  (bind _mat_for_obt_4 (`self.Mat for Obt_4`))
  (bind _mat_for_obt_5 (`self.Mat for Obt_5`))
  (bind _mat_for_obt_6 (`self.Mat for Obt_6`))
  (bind _mat_for_connection_1 (`self.Mat for Connection_1`))
  (bind _mat_for_connection_2 (`self.Mat for Connection_2`))
  (bind _mat_for_connection_3 (`self.Mat for Connection_3`))
  (bind _mat_for_obt_1 (`self.Mat for Obt_1`))
  ;[1 1 1] Mat Assign
  (`ActorComponent.SetActive` (`self.End_PS_1`) false false)
  (`ActorComponent.SetActive` (`self.End_PT_1`) false false)
  (`ActorComponent.SetActive` (`self.End_PS_2`) false false)
  (`ActorComponent.SetActive` (`self.End_PT_2`) false false)
  (`ActorComponent.SetActive` (`self.End_PS_3`) false false)
  (`ActorComponent.SetActive` (`self.End_PT_3`) false false)
  (`SceneComponent.SetVisibility` (`self.Cable_6`) false false)
  (`SceneComponent.SetVisibility` (`self.Cable_1_2`) false false)
  (`SceneComponent.SetVisibility` (`self.Cable_2_2`) false false)
  (`SceneComponent.SetVisibility` (`self.Cable_3_2`) false false)
  (`SceneComponent.SetVisibility` (`self.Cable_4_2`) false false)
  (`SceneComponent.SetVisibility` (`self.Cable_5_2`) false false)
  (`SceneComponent.SetVisibility` (`self.Cable_6_2`) false false)
  (`SceneComponent.SetVisibility` (`self.Cable_5`) false false)
  (`SceneComponent.SetVisibility` (`self.Cable_4`) false false)
  (`|ExecutionSequence`
    (:`then_1`
      (`PrimitiveComponent.SetMaterial` (`self.Start_1`) 0 _mat_for_start_1)
      (`PrimitiveComponent.SetMaterial` (`self.Cable_1`) 0 _mat_for_start_1)
      (`PrimitiveComponent.SetMaterial` (`self.Start_2`) 0 _mat_for_start_2)
      (`PrimitiveComponent.SetMaterial` (`self.Cable_2`) 0 _mat_for_start_2)
      (`PrimitiveComponent.SetMaterial` (`self.Start_3`) 0 _mat_for_start_3)
      (`PrimitiveComponent.SetMaterial` (`self.Cable_3`) 0 _mat_for_start_3)
      (`PrimitiveComponent.SetMaterial` (`self.Cable_1_2`) 0 _mat_for_obt_1)
      (`PrimitiveComponent.SetMaterial` (`self.1`) 0 _mat_for_obt_1)
      (`PrimitiveComponent.SetMaterial` (`self.Cable_2_2`) 0 _mat_for_obt_2)
      (`PrimitiveComponent.SetMaterial` (`self.2`) 0 _mat_for_obt_2)
      (`PrimitiveComponent.SetMaterial` (`self.Cable_3_2`) 0 _mat_for_obt_3)
      (`PrimitiveComponent.SetMaterial` (`self.3`) 0 _mat_for_obt_3)
      (`PrimitiveComponent.SetMaterial` (`self.Cable_4_2`) 0 _mat_for_obt_4)
      (`PrimitiveComponent.SetMaterial` (`self.4`) 0 _mat_for_obt_4)
      (`PrimitiveComponent.SetMaterial` (`self.Cable_5_2`) 0 _mat_for_obt_5)
      (`PrimitiveComponent.SetMaterial` (`self.5`) 0 _mat_for_obt_5)
      (`PrimitiveComponent.SetMaterial` (`self.Cable_6_2`) 0 _mat_for_obt_6)
      (`PrimitiveComponent.SetMaterial` (`self.6`) 0 _mat_for_obt_6)
      (`PrimitiveComponent.SetMaterial` (`self.Cable_4`) 0 _mat_for_connection_1)
      (`PrimitiveComponent.SetMaterial` (`self.Connector_1`) 0 _mat_for_connection_1)
      (`PrimitiveComponent.SetMaterial` (`self.Cable_5`) 0 _mat_for_connection_2)
      (`PrimitiveComponent.SetMaterial` (`self.Connector_2`) 0 _mat_for_connection_2)
      (`PrimitiveComponent.SetMaterial` (`self.Cable_6`) 0 _mat_for_connection_3)
      (`PrimitiveComponent.SetMaterial` (`self.Connector_3`) 0 _mat_for_connection_3)
      (`PrimitiveComponent.SetMaterial` (`self.End_1`) 0 (`self.Mat for End_1`))
      (`PrimitiveComponent.SetMaterial` (`self.End_2`) 0 (`self.Mat for End_2`))
      (`PrimitiveComponent.SetMaterial` (`self.End_3`) 0 (`self.Mat for End_3`))
      (bind _asnext_level_hud (cast `/Game/Jatin_Working_folder/HUD/Next_Level_HUD` (`PlayerController.GetHUD` (`GameplayStatics.GetPlayerController` 0)))))))

(fn `UserConstructionScript`)